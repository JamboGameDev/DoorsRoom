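; BP_Door1 is a swinging door that opens only for a BP_FirstPersonCharacter whose Cartinkey flag is set.
; Overlapping Box passes a DoOnce, plays a sound and runs a timeline that sets the Scene component's yaw.
; Leaving Box1 passes a second DoOnce, plays another sound and reverses the timeline after a short delay.
; The timeline's Finished output resets both DoOnce gates.
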(event OnComponentBeginOverlap(Box)
  (params (OverlappedComponent :type Primitive%20Component%20Object%20Reference) (OtherActor :type Actor%20Object%20Reference) (OtherComp :type Primitive%20Component%20Object%20Reference) (OtherBodyIndex :type Integer) (bFromSweep :type Boolean) (SweepResult :type Hit%20Result%20Structure%20%28by%20ref%29))
  ;[0 0 0] Дверь
  (bind _asbp_first_person_character (Utilities|Casting|CastToBP_FirstPersonCharacter OtherActor))
  (if (Variables|/Game/BP_Charector/BP_FirstPersonCharacter.BP_FirstPersonCharacter_C|GetCartinkey _asbp_first_person_character)
    (Utilities|FlowControl|DoOnce false :!label _label
      (:Completed
        (Audio|PlaySound2D "/Game/Asset_BP/Test_Mehanik/Asset_Saund/zvuk-dveri_jJtGwUQl_Cue.zvuk-dveri_jJtGwUQl_Cue" 1.0 1.0 0.0 0 0)
        (bind _lf (Timeline|Timeline Play)
          (:Update
            (Transformation|SetRelativeRotation (Variables|Default|GetScene) (Math|Rotator|MakeRotator 0.0 0.0 _lf) false false))
          (:Finished
            (Utilities|FlowControl|Sequence
              (:then_0
                (goto _label Reset))
              (:then_1
                (Utilities|FlowControl|DoOnce false) ; enters at Reset
              ))))))))

(event OnComponentEndOverlap(Box1)
  (params (OverlappedComponent :type Primitive%20Component%20Object%20Reference) (OtherActor :type Actor%20Object%20Reference) (OtherComp :type Primitive%20Component%20Object%20Reference) (OtherBodyIndex :type Integer))
  ;[0 0 0] Дверь
  (Utilities|Casting|CastToBP_FirstPersonCharacter OtherActor)
  (Utilities|FlowControl|DoOnce false :!label _label
    (:Completed
      (Audio|PlaySound2D "/Game/Asset_BP/Test_Mehanik/Asset_Saund/zvuk-dveri_Sd4C9r2e_Cue.zvuk-dveri_Sd4C9r2e_Cue" 1.0 1.0 0.0 0 0)
      (Utilities|FlowControl|Delay 0.5)
      (bind _lf (Timeline|Timeline Reverse)
        (:Update
          (Transformation|SetRelativeRotation (Variables|Default|GetScene) (Math|Rotator|MakeRotator 0.0 0.0 _lf) false false))
        (:Finished
          (Utilities|FlowControl|Sequence
            (:then_0
              (Utilities|FlowControl|DoOnce false) ; enters at Reset
            )
            (:then_1
              (goto _label Reset))))))))

(fn ConstructionScript)