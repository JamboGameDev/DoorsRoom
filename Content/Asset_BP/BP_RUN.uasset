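; BP_RUN is an energy drink pickup that gives the first-person player a temporary speed boost.
; Sphere overlap fires once, plays a sound and raises walk speed by an amount depending on the crouch flag.
; When standing, a Timeline widens the camera FOV, and its update hides the light and feeds the timed reset.
; After the delay it restores speed for the current stance, reverses the FOV if standing, and destroys itself.
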(event OnComponentBeginOverlap(Sphere)
  (params (OverlappedComponent :type Primitive%20Component%20Object%20Reference) (OtherActor :type Actor%20Object%20Reference) (OtherComp :type Primitive%20Component%20Object%20Reference) (OtherBodyIndex :type Integer) (bFromSweep :type Boolean) (SweepResult :type Hit%20Result%20Structure%20%28by%20ref%29))
  ;[0 0 0] Проверка Енергоса
  (bind _asbp_first_person_character (Utilities|Casting|CastToBP_FirstPersonCharacter OtherActor))
  (Variables|Default|Setwon true)
  (bind _output_get (Variables|Default|SetPlayerRF _asbp_first_person_character))
  (if (Variables|Default|Getwon)
    (Utilities|FlowControl|DoOnce false
      (:Completed
        (Audio|PlaySound2D "/Game/Asset_BP/Test_Mehanik/Asset_Saund/run.run" 1.0 1.0 0.0 0 0)
        (if (Variables|/Game/BP_Charector/BP_FirstPersonCharacter.BP_FirstPersonCharacter_C|GetCroch _asbp_first_person_character)
          (Variables|/Game/BP_Charector/BP_FirstPersonCharacter.BP_FirstPersonCharacter_C|SetCroch _asbp_first_person_character true)
          (Variables|/Script/Engine.CharacterMovementComponent|SetMaxWalkSpeed (Variables|/Script/Engine.Character|GetCharacterMovement _asbp_first_person_character) 3e+02)
          (Rendering|SetVisibility (Variables|Default|GetFleshLight) false false :!label _label)
          (Utilities|FlowControl|Delay 5.0)
          (if (Variables|/Game/BP_Charector/BP_FirstPersonCharacter.BP_FirstPersonCharacter_C|GetCroch _asbp_first_person_character)
            (Variables|/Game/BP_Charector/BP_FirstPersonCharacter.BP_FirstPersonCharacter_C|SetCroch _asbp_first_person_character true)
            (Variables|/Script/Engine.CharacterMovementComponent|SetMaxWalkSpeed (Variables|/Script/Engine.Character|GetCharacterMovement _asbp_first_person_character) 1.5e+02)
            (Actor|DestroyActor :!label _label_2)
            (else
              (Variables|/Game/BP_Charector/BP_FirstPersonCharacter.BP_FirstPersonCharacter_C|SetCroch _asbp_first_person_character false)
              (Variables|/Script/Engine.CharacterMovementComponent|SetMaxWalkSpeed (Variables|/Script/Engine.Character|GetCharacterMovement _asbp_first_person_character) 4e+02)
              (Utilities|FlowControl|Sequence
                (:then_0
                  (Utilities|FlowControl|Delay 5.1)
                  (goto _label_2))
                (:then_1
                  (bind _newtrack_1 (Timeline|Timeline Reverse)
                    (:Update
                      (Utilities|FlowControl|Sequence
                        (:then_0
                          (Camera|SetFieldOfView (Variables|/Game/BP_Charector/BP_FirstPersonCharacter.BP_FirstPersonCharacter_C|GetCamera1 _asbp_first_person_character) (Math|Float|Lerp 9e+01 1.1e+02 _newtrack_1)))
                        (:then_1
                          (Transformation|AttachComponentToComponent (Variables|/Script/Engine.Actor|GetRootComponent _output_get) 0 "None" "KeepRelative" "KeepRelative" "KeepRelative" true)
                          (goto _label)))))))))
          (else
            (Variables|/Game/BP_Charector/BP_FirstPersonCharacter.BP_FirstPersonCharacter_C|SetCroch _asbp_first_person_character false)
            (Variables|/Script/Engine.CharacterMovementComponent|SetMaxWalkSpeed (Variables|/Script/Engine.Character|GetCharacterMovement _asbp_first_person_character) 7e+02)
            (Timeline|Timeline Play)))))))

(fn ConstructionScript)