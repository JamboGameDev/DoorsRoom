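; BP_MonsterSimple is a test monster that makes a one-time dash when the player enters its Box trigger.
; The first player overlap plays a dying-breath sound, then after a short delay a Timeline lerps the actor far along negative world X, with Z set to zero.
; Box1's overlap only casts to the player character, as the death-widget and input-disable logic is left unconnected.
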(event OnComponentBeginOverlap(Box)
  (params (OverlappedComponent :type Primitive%20Component%20Object%20Reference) (OtherActor :type Actor%20Object%20Reference) (OtherComp :type Primitive%20Component%20Object%20Reference) (OtherBodyIndex :type Integer) (bFromSweep :type Boolean) (SweepResult :type Hit%20Result%20Structure%20%28by%20ref%29))
  (bind _returnvalue (Transformation|GetActorLocation))
  (Utilities|Casting|CastToBP_FirstPersonCharacter OtherActor)
  (Utilities|FlowControl|DoOnce false
    (:Completed
      (Audio|PlaySound2D "/Game/Asset_BP/Test_Mehanik/Asset_Saund/woman39s-dying-breath_TBYAKfj3_Cue.woman39s-dying-breath_TBYAKfj3_Cue" 1.0 1.0 0.0 0 0)
      (Utilities|FlowControl|Delay 0.6)
      (bind _output_get (Variables|Default|SetStartLocation (Math|Vector|MakeVector (.x _returnvalue) (.y _returnvalue) 0.0)))
      (bind _newtrack_0 (Timeline|Timeline Play)
        (:Update
          (Transformation|SetActorLocation (Math|Vector|MakeVector (Math|Float|Lerp (.x _output_get) (+ (.x _output_get) -1e+04) _newtrack_0) (.y _output_get) 0.0) false false))))))

(event OnComponentBeginOverlap(Box1)
  (params (OverlappedComponent :type Primitive%20Component%20Object%20Reference) (OtherActor :type Actor%20Object%20Reference) (OtherComp :type Primitive%20Component%20Object%20Reference) (OtherBodyIndex :type Integer) (bFromSweep :type Boolean) (SweepResult :type Hit%20Result%20Structure%20%28by%20ref%29))
  (Utilities|Casting|CastToBP_FirstPersonCharacter OtherActor))

(event EventBeginPlay)

(event Collision|EventActorBeginOverlap
  (params (OtherActor :type Actor%20Object%20Reference)))

(fn ConstructionScript)