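; BP_Door2 is a key-locked door that swings open once and closes behind the player.
; EventInteract checks PikKey on the first-person character, then plays a sound and a Timeline that drives Scene's yaw.
; When the character leaves Box1, IsopenDooer2 is set, blocking further opening, and the Timeline reverses with a closing sound.
; DoOnce nodes limit opening and closing to a single time each.
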(event OnComponentEndOverlap(Box1)
  (params (OverlappedComponent :type Primitive%20Component%20Object%20Reference) (OtherActor :type Actor%20Object%20Reference) (OtherComp :type Primitive%20Component%20Object%20Reference) (OtherBodyIndex :type Integer))
  ;[0 0 0] Дверь
  (Utilities|Casting|CastToBP_FirstPersonCharacter OtherActor)
  (Variables|Default|SetIsopenDooer2 true)
  (Utilities|FlowControl|DoOnce false
    (:Completed
      (Utilities|FlowControl|Sequence
        (:then_0
          (bind _lf (Timeline|Timeline Reverse)
            (:Update
              (Transformation|SetRelativeRotation (Variables|Default|GetScene) (Math|Rotator|MakeRotator 0.0 0.0 _lf) false false))))
        (:then_1
          (Audio|PlaySound2D "/Game/Asset_BP/Test_Mehanik/Asset_Saund/zvuk-dveri_Sd4C9r2e_Cue.zvuk-dveri_Sd4C9r2e_Cue" 1.0 1.0 0.0 0 0))))))

(event EventEventInteract
  ;[0 0 0] Дверь
  (bind _asbp_first_person_character (Utilities|Casting|CastToBP_FirstPersonCharacter (Game|GetPlayerCharacter 0)))
  (if (Variables|/Game/BP_Charector/BP_FirstPersonCharacter.BP_FirstPersonCharacter_C|GetPik%20key _asbp_first_person_character)
    (if (not (Variables|Default|GetIsopenDooer2))
      (Utilities|FlowControl|DoOnce false
        (:Completed
          (Audio|PlaySound2D "/Game/Asset_BP/Test_Mehanik/Asset_Saund/zvuk-dveri_jJtGwUQl_Cue.zvuk-dveri_jJtGwUQl_Cue" 1.0 1.0 0.0 0 0)
          (bind _lf (Timeline|Timeline Play)
            (:Update
              (Transformation|SetRelativeRotation (Variables|Default|GetScene) (Math|Rotator|MakeRotator 0.0 0.0 _lf) false false))))))))

(fn ConstructionScript)