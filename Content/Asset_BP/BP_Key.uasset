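; BP_Key is a key pickup actor that sets the PikKey flag on BP_FirstPersonCharacter when the player overlaps its Box.
; A separate Box1 overlap plays a one-time timeline that drives the point light's intensity.
; Pickup sets Svet, attaches the Sphere and reverses that timeline, whose update then hides the Sphere, plays a sound once and destroys the actor after a short delay.
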(event OnComponentBeginOverlap(Box1)
  (params (OverlappedComponent :type Primitive%20Component%20Object%20Reference) (OtherActor :type Actor%20Object%20Reference) (OtherComp :type Primitive%20Component%20Object%20Reference) (OtherBodyIndex :type Integer) (bFromSweep :type Boolean) (SweepResult :type Hit%20Result%20Structure%20%28by%20ref%29))
  ;[0 0 0] подбор
  (Utilities|Casting|CastToBP_FirstPersonCharacter OtherActor)
  (Utilities|FlowControl|DoOnce false
    (:Completed
      (bind _newtrack_0 (Timeline|Timeline Play)
        (:Update
          (Rendering|Components|Light|SetIntensity (Variables|Default|GetPointLight) _newtrack_0)
          (if (Variables|Default|GetSvet)
            (Rendering|SetVisibility (Variables|Default|GetSphere) false false)
            (Utilities|FlowControl|DoOnce false
              (:Completed
                (Audio|PlaySound2D "/Game/Asset_BP/Test_Mehanik/Asset_Saund/1563696141-0ad40b709c395ea_L3Pp0vT4_Cue.1563696141-0ad40b709c395ea_L3Pp0vT4_Cue" 1.0 1.0 0.0 0 0)
                (Utilities|FlowControl|Delay 3.0)
                (Actor|DestroyActor)))))))))

(event OnComponentBeginOverlap(Box)
  (params (OverlappedComponent :type Primitive%20Component%20Object%20Reference) (OtherActor :type Actor%20Object%20Reference) (OtherComp :type Primitive%20Component%20Object%20Reference) (OtherBodyIndex :type Integer) (bFromSweep :type Boolean) (SweepResult :type Hit%20Result%20Structure%20%28by%20ref%29))
  ;[0 0 0] подбор
  (bind _asbp_first_person_character (Utilities|Casting|CastToBP_FirstPersonCharacter OtherActor))
  (Variables|/Game/BP_Charector/BP_FirstPersonCharacter.BP_FirstPersonCharacter_C|SetPik%20key _asbp_first_person_character true)
  (Variables|Default|SetSvet true)
  (Transformation|AttachComponentToComponent (Variables|Default|GetSphere) 0 "None" "KeepRelative" "KeepRelative" "KeepRelative" true)
  (bind _newtrack_0 (Timeline|Timeline Reverse)
    (:Update
      (Rendering|Components|Light|SetIntensity (Variables|Default|GetPointLight) _newtrack_0)
      (if (Variables|Default|GetSvet)
        (Rendering|SetVisibility (Variables|Default|GetSphere) false false)
        (Utilities|FlowControl|DoOnce false
          (:Completed
            (Audio|PlaySound2D "/Game/Asset_BP/Test_Mehanik/Asset_Saund/1563696141-0ad40b709c395ea_L3Pp0vT4_Cue.1563696141-0ad40b709c395ea_L3Pp0vT4_Cue" 1.0 1.0 0.0 0 0)
            (Utilities|FlowControl|Delay 3.0)
            (Actor|DestroyActor)))))))

(fn ConstructionScript)