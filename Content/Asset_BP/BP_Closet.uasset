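; BP_Closet is an interactable closet that the player can step into and out of, likely for hiding.
; EventInteract flip-flops between entering, which blends the view to the closet and disables movement, and exiting, which restores view and walking.
; Each transition plays a sound and two timelines that rotate the doors open, then reverse them shut after a short delay.
; DoOnce gates, reset as the doors start closing, and boolean flags limit retriggering.
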(event EventEventInteract
  (bind _returnvalue (Game|GetPlayerCharacter 0))
  (bind _returnvalue_2 (Game|GetPlayerController 0))
  ;[0 0 0] Отурытие
  (Utilities|FlowControl|FlipFlop
    (:A
      (Utilities|FlowControl|DoOnce false :!label _label
        (:Completed
          (Variables|Default|SetNewVar_1 true)
          (Game|Player|SetViewTargetwithBlend _returnvalue_2 self 0.8 "VTBlend_Linear" 0.8 false)
          (Input|SetIgnoreLookInput _returnvalue_2 false)
          (Pawn|Components|CharacterMovement|DisableMovement (Variables|/Script/Engine.Character|GetCharacterMovement (Game|GetPlayerCharacter 0)))
          (Audio|PlaySound2D "/Game/Asset_BP/Test_Mehanik/Asset_Saund/d5b2c99d5e5d79c_Cue.d5b2c99d5e5d79c_Cue" 1.0 1.0 0.0 0 0)
          (Variables|Default|SetNewVar true)
          (Variables|Default|SetNewVar_0 true)
          (Utilities|FlowControl|Sequence
            (:then_0
              (bind _lf (Timeline|Timeline Play)
                (:Update
                  (Transformation|SetRelativeRotation (Variables|Default|GetScene) (Math|Rotator|MakeRotator 0.0 0.0 _lf) false false))
                (:Finished
                  (if (Variables|Default|GetNewVar_0)
                    (Utilities|FlowControl|Delay 0.1)
                    (Variables|Default|SetNewVar_0 false)
                    (Utilities|FlowControl|Sequence
                      (:then_0
                        (Timeline|Timeline ReverseFromEnd))
                      (:then_1
                        (goto _label Reset)))))))
            (:then_1
              (bind _lf_2 (Timeline|Timeline_0 Play)
                (:Update
                  (Transformation|SetRelativeRotation (Variables|Default|GetScene1) (Math|Rotator|MakeRotator 0.0 0.0 _lf_2) false false))
                (:Finished
                  (if (Variables|Default|GetNewVar)
                    (Utilities|FlowControl|Delay 0.1)
                    (Variables|Default|SetNewVar false)
                    (Utilities|FlowControl|Sequence
                      (:then_0
                        (Timeline|Timeline_0 ReverseFromEnd))
                      (:then_1
                        (goto _label_2 Reset)))))))))))
    (:B
      (if (Variables|Default|GetNewVar_1)
        (Utilities|FlowControl|DoOnce false :!label _label_2
          (:Completed
            (Variables|Default|SetNewVar_1 false)
            (Game|Player|SetViewTargetwithBlend (Game|GetPlayerController 0) _returnvalue 0.8 "VTBlend_Linear" 0.8 false)
            (Input|ResetIgnoreLookInput _returnvalue_2)
            (Pawn|Components|CharacterMovement|SetMovementMode (Variables|/Script/Engine.Character|GetCharacterMovement _returnvalue) "MOVE_Walking" 0)
            (Audio|PlaySound2D "/Game/Asset_BP/Test_Mehanik/Asset_Saund/b8ff3214f634006_Cue.b8ff3214f634006_Cue" 1.0 1.0 0.0 0 0)
            (Variables|Default|SetNewVar true)
            (Variables|Default|SetNewVar_0 true)
            (Utilities|FlowControl|Sequence
              (:then_0
                (Timeline|Timeline Play))
              (:then_1
                (Timeline|Timeline_0 Play)))))))))

(fn ConstructionScript)